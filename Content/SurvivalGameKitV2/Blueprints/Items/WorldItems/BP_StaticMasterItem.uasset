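; Master world actor for static survival-kit inventory items, taking its mesh, offsets, name and available actions from item data.
; An SGK interface routes interactions to pickup, equip, open, consume, hold or learn, usually destroying the actor on success.
; TempItem holds created, dropped or loaded item state for saving and timed decay into replacement items.
; Contained inventories replicate only while players are nearby, and dropped items can self-destruct on a timer.
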(event `DropDestroyTimer`
  (`self.K2_DestroyActor`))

(event `/Game/SurvivalGameKitV2/Blueprints/Other/Interfaces/BP_SGKInteractionInterface.SGK PlayerInProximity`
  ;[1 1 1] Networking
  (bind _output_get (set `self.InvItem` (`self.TempItem`)))
  (bind ((`MasterInventory_8_17FFB7D341FAF2689C1BABA12E3BA9F5` _masterinventory)) (break `/Game/SurvivalGameKitV2/Blueprints/Other/Structs/S_InvItem` _output_get))
  (`/Engine/EditorBlueprintResources/StandardMacros.IsValid` _masterinventory
    (:`Is Valid`
      (if (not (`ActorComponent.bReplicates` _masterinventory))
        (`/Game/SurvivalGameKitV2/Blueprints/Components/BP_MasterInventory.ReplicateContainingInventories` _masterinventory true)))))

(event `/Game/SurvivalGameKitV2/Blueprints/Other/Interfaces/BP_SGKInteractionInterface.SGK PlayerOutProximity`
  (bind ((`ID_2_84C2CB8945979246059C568DCD463423` _id) (`MasterInventory_8_17FFB7D341FAF2689C1BABA12E3BA9F5` _masterinventory)) (break `/Game/SurvivalGameKitV2/Blueprints/Other/Structs/S_InvItem` (`self.InvItem`)))
  ;[1 1 1] Networking
  (`/Engine/EditorBlueprintResources/StandardMacros.IsValid` _masterinventory
    (:`Is Valid`
      (if (`ActorComponent.bReplicates` _masterinventory)
        (`/Engine/EditorBlueprintResources/StandardMacros.DoOnce` false :!label _label
          (:`Completed`
            (`|ExecutionSequence`
              (:`then_0`
                (bind (_outactors _returnvalue) (`KismetSystemLibrary.SphereOverlapActors` (`self.K2_GetActorLocation`) 600.0 (`|MakeArray` "ObjectTypeQuery3" :!type "EObjectTypeQuery Enum") "/Script/Engine.Character"))
                (if (not _returnvalue)
                  (`/Game/SurvivalGameKitV2/Blueprints/Components/BP_MasterInventory.ReplicateContainingInventories` (`.MasterInventory_8_17FFB7D341FAF2689C1BABA12E3BA9F5` (break `/Game/SurvivalGameKitV2/Blueprints/Other/Structs/S_InvItem` (`self.InvItem`))) false)))
              (:`then_1`
                (`KismetSystemLibrary.Delay` 0.5)
                (`self.Reset`)))))))))

(event `Reset`
  ;[1 1 1] Networking
  (goto _label :!via `Reset`))

(event `self.ReceiveBeginPlay`
  ;[1 1 1] Begin Play
  (`parent.ReceiveBeginPlay`)
  (if (`KismetSystemLibrary.IsStandalone`)
    (set `self.TempItem` (`self.InvItem`) :!label _label_2)
    (elif (`self.SaveGameLoaded`)
      _
      (else
        (goto _label_2))))
  (`/Engine/EditorBlueprintResources/ActorMacros.Switch Has Authority`
    (:`Authority`
      (bind _savegame (message `/Game/SurvivalGameKitV2/Blueprints/Other/Interfaces/BP_SGKGameModeInterface.SGK GetSaveGame` (`GameplayStatics.GetGameMode`)))
      (bind _output_get (set `self.SaveGame` _savegame))
      (`/Engine/EditorBlueprintResources/StandardMacros.IsValid` _output_get
        (:`Is Valid`
          (add `/Game/SurvivalGameKitV2/Blueprints/Saving/BP_SaveSystem.LoadData` (`self.SaveGame`) (delegate `LoadItem`))
          (add `/Game/SurvivalGameKitV2/Blueprints/Saving/BP_SaveSystem.SaveData` (`self.SaveGame`) (delegate `SaveItem`))
          (`/Engine/EditorBlueprintResources/StandardMacros.IsValid` (`self.GetOwner`)
            (:`Is Not Valid`
              (if (`/Game/SurvivalGameKitV2/Blueprints/Saving/BP_SaveSystem.FirstLoadDone` (`self.SaveGame`))
                (if (or (`self.Spawned`) (`self.Dropped`))
                  (`|ExecutionSequence` :!label _label_3
                    (:`then_0`
                      (bind _asbp_sgkgame_mode (cast `/Game/SurvivalGameKitV2/Blueprints/Characters/BP_SGKGameMode` (`GameplayStatics.GetGameMode`)))
                      (add `/Game/SurvivalGameKitV2/Blueprints/Characters/BP_SGKGameMode.CreateInventory` _asbp_sgkgame_mode (delegate `CreateNewItem`)))
                    (:`then_1`
                      (`StaticMeshComponent.SetStaticMesh` (`self.StaticMesh`) (`.StaticMesh_30_DB8565E8487831578F6D18823B88B876` (break `/Game/SurvivalGameKitV2/Blueprints/Other/Structs/S_ItemDetails` (`.ItemDetails` (`/Game/SurvivalGameKitV2/Blueprints/Other/Interfaces/BP_SGKFunctions.SGK ItemDetails` (`self.InvItem`)))))))
                    (:`then_2`
                      (`KismetSystemLibrary.Delay` (`KismetMathLibrary.RandomFloatInRange` 0.0 0.2))
                      (if (`.UseItemDecay_1_12FBBE5940F95B2CAFEB29B32812EBC0` (break `/Game/SurvivalGameKitV2/Blueprints/Other/Structs/S_DecayDetails` (`.DecayDetails_28_E55B8B1D423F7D487FFACDAB43C68F74` (break `/Game/SurvivalGameKitV2/Blueprints/Other/Structs/S_DurabilityDetails` (`.DurabilityDetails` (`/Game/SurvivalGameKitV2/Blueprints/Other/Interfaces/BP_SGKFunctions.SGK DurabilityDetails` (`self.TempItem`)))))))
                        (`KismetSystemLibrary.K2_SetTimer` null "ItemDecay" 60.0 true))))
                  (elif (not (`self.SaveGameLoaded`))
                    (`self.K2_DestroyActor`)))
                (else
                  (goto _label_3))))))
        (:`Is Not Valid`
          (`self.SaveNotValid`))))))

(event `CreateNewItem`
  (bind (_id _amount) (break `/Game/SurvivalGameKitV2/Blueprints/Other/Structs/S_InvItem` (`self.InvItem`)))
  ;[1 1 1] Begin Play
  (bind _globalinventory (message `/Game/SurvivalGameKitV2/Blueprints/Other/Interfaces/BP_SGKGameModeInterface.SGK GetGlobalInventory` (`GameplayStatics.GetGameMode`)))
  (bind _newitem (`/Game/SurvivalGameKitV2/Blueprints/Other/BP_GlobalInventoryManager.CreateNewItem` _globalinventory _id _amount true true false false))
  (set `self.TempItem` _newitem)
  (if (`KismetSystemLibrary.IsStandalone`)
    (set `self.InvItem` (`self.TempItem`))))

(event `SaveItem`
  (params (SaveGame :type "/Game/SurvivalGameKitV2/Blueprints/Saving/BP_SGKSaveGame Object Reference"))
  ;[1 1 1] Begin Play
  (if (not (`self.Spawned`))
    (bind _returnvalue (`GameplayStatics.GetCurrentLevelName` true))
    (`/Game/SurvivalGameKitV2/Blueprints/Saving/BP_SGKSaveGame.SaveItem` SaveGame (`self.GetTransform`) (`self.TempItem`) _returnvalue)))

(event `LoadItem`
  (params (SaveGame :type "/Game/SurvivalGameKitV2/Blueprints/Saving/BP_SGKSaveGame Object Reference"))
  ;[1 1 1] Begin Play
  (`self.K2_DestroyActor`))

(event `SaveNotValid`
  ;[1 1 1] Begin Play
  (`/Engine/EditorBlueprintResources/StandardMacros.IsValid` (`self.GetOwner`)
    (:`Is Not Valid`
      (goto _label_3))))

(fn `Consume`
  (params (PlayerInventory :type "/Game/SurvivalGameKitV2/Blueprints/Components/BP_PlayerInventory Object Reference"))
  (locals (ConsumedItemL :type "/Game/SurvivalGameKitV2/Blueprints/Other/Structs/S_InvItem Structure"))
  (bind _consumediteml (`local.ConsumedItemL`))
  ;[1 1 1] Consume item
  (bind _consumed (`/Game/SurvivalGameKitV2/Blueprints/Components/BP_PlayerInventory.ConsumeItem` (`local.PlayerInventory`) (`self.InvItem`)))
  (if _consumed
    ;[1 1 1] Remove use item amount
    (bind (_itemempty _itemout) (`/Game/SurvivalGameKitV2/Blueprints/Components/BP_PlayerInventory.UpdateItemUseAmount` (`local.PlayerInventory`) (`self.InvItem`) -1))
    (set `local.ConsumedItemL` _itemout)
    (if _itemempty
      ;[1 1 1] If used up destroy actor
      (`self.K2_DestroyActor`)
      (else
        ;[1 1 1] If use item amount remaining set new amount
        (set `self.InvItem` _consumediteml)
        (set `self.TempItem` _consumediteml)))))

(fn `EquipClothing`
  (params (PlayerInventory :type "/Game/SurvivalGameKitV2/Blueprints/Components/BP_PlayerInventory Object Reference"))
  (bind (_invitem_id _invitem_amount _invitem_masterinventory) (break `/Game/SurvivalGameKitV2/Blueprints/Other/Structs/S_InvItem` (`self.InvItem`)))
  ;[1 1 1] Attempt to equip the item as clothing if equipped destroy actor
  (bind _itemequipped (`/Game/SurvivalGameKitV2/Blueprints/Components/BP_PlayerInventory.AttemptToEquipItem` (`local.PlayerInventory`) (`self.InvItem`)))
  (if _itemequipped
    (`self.K2_DestroyActor`)
    ;[1 1 1] Close other players using the inventory
    (`/Engine/EditorBlueprintResources/StandardMacros.IsValid` _invitem_masterinventory
      (:`Is Valid`
        (`/Game/SurvivalGameKitV2/Blueprints/Components/BP_MasterInventory.CloseOtherPlayerTabs` _invitem_masterinventory (`local.PlayerInventory`))))))

(fn `EquipWeapon`
  (params (PlayerInventory :type "/Game/SurvivalGameKitV2/Blueprints/Components/BP_PlayerInventory Object Reference"))
  (bind (_invitem_id _invitem_amount _invitem_masterinventory) (break `/Game/SurvivalGameKitV2/Blueprints/Other/Structs/S_InvItem` (`self.InvItem`)))
  ;[1 1 1] Attempt to equip item to weapon slot and if equipped destroy actor
  (bind _weaponequipped (`/Game/SurvivalGameKitV2/Blueprints/Components/BP_PlayerInventory.AttemptToEquipWeapon` (`local.PlayerInventory`) (`self.InvItem`) true))
  (if _weaponequipped
    (`self.K2_DestroyActor`)
    ;[1 1 1] Close other players using the inventory
    (`/Engine/EditorBlueprintResources/StandardMacros.IsValid` _invitem_masterinventory
      (:`Is Valid`
        (`/Game/SurvivalGameKitV2/Blueprints/Components/BP_MasterInventory.CloseOtherPlayerTabs` _invitem_masterinventory (`local.PlayerInventory`))))))

(fn `Hold`
  (params (PlayerInventory :type "/Game/SurvivalGameKitV2/Blueprints/Components/BP_PlayerInventory Object Reference"))
  ;[1 1 1] Attempt to hold item and if held destroy actor
  (bind (_itemheld _itemadded) (`/Game/SurvivalGameKitV2/Blueprints/Components/BP_PlayerInventory.AttemptToPickupHold` (`local.PlayerInventory`) (`self.InvItem`)))
  (if _itemadded
    (`self.K2_DestroyActor`)))

(fn `Interact`
  (params (PlayerInventory :type "/Game/SurvivalGameKitV2/Blueprints/Components/BP_PlayerInventory Object Reference"))
  ;[1 1 1] Can be expanded or overriden
  (`KismetSystemLibrary.PrintString` "ERROR :: No functionaliy set in Interact function in the \nBP_MasterStaticItem" true true (struct :`R` 1.0 :`B` 0.137618 :`A` 1.0) 10.0))

(fn `InteractActions`
  (params (PlayerInventory :type "/Game/SurvivalGameKitV2/Blueprints/Components/BP_PlayerInventory Object Reference") (Action :type "/Game/SurvivalGameKitV2/Blueprints/Other/Enum/E_WorldActions Enum" :default "NewEnumerator0"))
  (locals (StartAmountL :type Integer))
  (bind ((`ShortName_53_3FDED9954C8DBFC313F77D9D147163D6` _shortname) (`PickupAnimation_119_0B5E9F0B4C814F6522050FB1A71E95A6` _pickupanimation)) (break `/Game/SurvivalGameKitV2/Blueprints/Other/Structs/S_ItemDetails` (`.ItemDetails` (`/Game/SurvivalGameKitV2/Blueprints/Other/Interfaces/BP_SGKFunctions.SGK ItemDetails` (`self.InvItem`)))))
  (if (not (`KismetSystemLibrary.IsStandalone`))
    ;[1 1 1] If loaded from save then set inv item
    (if (`self.SaveGameLoaded`)
      (set `self.InvItem` (`self.TempItem`))))
  (switch `/Game/SurvivalGameKitV2/Blueprints/Other/Enum/E_WorldActions` (`local.Action`)
    (:`NewEnumerator8`
      ;[1 1 1] Call action events
      (`self.Interact` (`local.PlayerInventory`)))
    (:`NewEnumerator1`
      (`self.Pickup` (`local.PlayerInventory`))
      ;[1 1 1] Call multicast play pickup animation for item
      (`/Engine/EditorBlueprintResources/StandardMacros.IsValid` _pickupanimation :!label _label
        (:`Is Valid`
          (`/Game/SurvivalGameKitV2/Blueprints/Components/BP_CharacterComponent.MulticastPlayMontage` (`/Game/SurvivalGameKitV2/Blueprints/Components/BP_PlayerInventory.CharacterComponent` (`local.PlayerInventory`)) _pickupanimation null))))
    (:`NewEnumerator2`
      (`self.EquipClothing` (`local.PlayerInventory`))
      (goto _label))
    (:`NewEnumerator3`
      (`self.Open` (`local.PlayerInventory`)))
    (:`NewEnumerator4`
      (`self.EquipWeapon` (`local.PlayerInventory`))
      (goto _label))
    (:`NewEnumerator5`
      (`self.Consume` (`local.PlayerInventory`))
      (goto _label))
    (:`NewEnumerator6`
      (`self.Hold` (`local.PlayerInventory`)))
    (:`NewEnumerator7`
      (`self.Learn` (`local.PlayerInventory`)))))

(fn `ItemDecay`
  (locals (DecayDetailsL :type "/Game/SurvivalGameKitV2/Blueprints/Other/Structs/S_DecayDetails Structure" :default (struct :`DecayTimeMinutes` 30 :`ReplacementItem` (struct :`DataTable` "CompositeDataTable'\"/Game/SurvivalGameKitV2/Blueprints/Items/MasterLists/MasterItemList.MasterItemList\"'"))))
  (bind ((`MasterInventory_8_17FFB7D341FAF2689C1BABA12E3BA9F5` _masterinventory)) (break `/Game/SurvivalGameKitV2/Blueprints/Other/Structs/S_InvItem` (`self.TempItem`)))
  (bind ((`MasterInventory_8_17FFB7D341FAF2689C1BABA12E3BA9F5` _masterinventory_2)) (break `/Game/SurvivalGameKitV2/Blueprints/Other/Structs/S_InvItem` (`self.TempItem`)))
  (bind ((`DecayDetails_28_E55B8B1D423F7D487FFACDAB43C68F74` _decaydetails)) (break `/Game/SurvivalGameKitV2/Blueprints/Other/Structs/S_DurabilityDetails` (`.DurabilityDetails` (`/Game/SurvivalGameKitV2/Blueprints/Other/Interfaces/BP_SGKFunctions.SGK DurabilityDetails` (`self.TempItem`)))))
  (bind (_datatable _rowname) (break `DataTableRowHandle` (`.ReplacementItem_8_29EAE32547957C641D561A99857A2984` (break `/Game/SurvivalGameKitV2/Blueprints/Other/Structs/S_DecayDetails` (`local.DecayDetailsL`)))))
  (bind _returnvalue (- (`.DecayTime_33_E35E189B4E5F129EEECA28AE05E99A93` (break `/Game/SurvivalGameKitV2/Blueprints/Other/Structs/S_InvItem` (`self.TempItem`))) 1))
  (set `local.DecayDetailsL` _decaydetails)
  (if (and (`.UseItemDecay_1_12FBBE5940F95B2CAFEB29B32812EBC0` (break `/Game/SurvivalGameKitV2/Blueprints/Other/Structs/S_DecayDetails` _decaydetails)) (not (`.AllowStacking_48_02CFD0D74B05709E8E432E824709C714` (break `/Game/SurvivalGameKitV2/Blueprints/Other/Structs/S_ItemDetails` (`.ItemDetails` (`/Game/SurvivalGameKitV2/Blueprints/Other/Interfaces/BP_SGKFunctions.SGK ItemDetails` (`self.TempItem`)))))))
    (if (<= _returnvalue 0)
      (if (`/Game/SurvivalGameKitV2/Blueprints/Other/Interfaces/BP_SGKFunctions.SGK ItemDetails` (make `/Game/SurvivalGameKitV2/Blueprints/Other/Structs/S_InvItem` _rowname))
        (bind _globalinventory (message `/Game/SurvivalGameKitV2/Blueprints/Other/Interfaces/BP_SGKGameModeInterface.SGK GetGlobalInventory` (`GameplayStatics.GetGameMode`)))
        (bind _newitem (`/Game/SurvivalGameKitV2/Blueprints/Other/BP_GlobalInventoryManager.CreateNewItem` _globalinventory _rowname 1 false false false true))
        (bind _returnvalue_2 (`|SpawnActorFromClass` (`.WorldClass_45_6718387F4F5D57BE9909639A237E57A3` (break `/Game/SurvivalGameKitV2/Blueprints/Other/Structs/S_ItemDetails` (`.ItemDetails` (`/Game/SurvivalGameKitV2/Blueprints/Other/Interfaces/BP_SGKFunctions.SGK ItemDetails` _newitem)))) (`self.GetTransform`) "AlwaysSpawn" "OverrideRootScale" (`self.GetOwner`) (`self.GetInstigator`)))
        (`/Engine/EditorBlueprintResources/StandardMacros.IsValid` _returnvalue_2
          (:`Is Valid`
            (message `/Game/SurvivalGameKitV2/Blueprints/Other/Interfaces/BP_SGKInteractionInterface.SGK DropItem` _returnvalue_2 _newitem false true false))
          (:`Is Not Valid`
            _))
        (if (`.DestroyOnDecay_5_6D147CB247BC631892F003AE614B8A5C` (break `/Game/SurvivalGameKitV2/Blueprints/Other/Structs/S_DecayDetails` (`local.DecayDetailsL`)))
          (`/Engine/EditorBlueprintResources/StandardMacros.IsValid` _masterinventory
            (:`Is Valid`
              (`/Game/SurvivalGameKitV2/Blueprints/Components/BP_MasterInventory.DestroyContainingInventories` _masterinventory)
              (`ActorComponent.K2_DestroyComponent` _masterinventory))
            (:`Is Not Valid`
              _))
          (`self.K2_DestroyActor`))
        (elif (`.DestroyOnDecay_5_6D147CB247BC631892F003AE614B8A5C` (break `/Game/SurvivalGameKitV2/Blueprints/Other/Structs/S_DecayDetails` (`local.DecayDetailsL`)))
          (`/Engine/EditorBlueprintResources/StandardMacros.IsValid` _masterinventory_2
            (:`Is Valid`
              (`/Game/SurvivalGameKitV2/Blueprints/Components/BP_MasterInventory.DestroyContainingInventories` _masterinventory_2)
              (`ActorComponent.K2_DestroyComponent` _masterinventory_2))
            (:`Is Not Valid`
              _))
          (`self.K2_DestroyActor`)))
      (else
        (setmembers `/Game/SurvivalGameKitV2/Blueprints/Other/Structs/S_InvItem` :`StructRef` (`self.TempItem`) :`DecayTime` _returnvalue)))))

(fn `ItemOffsets`
  (locals (ItemDetailsL :type "/Game/SurvivalGameKitV2/Blueprints/Other/Structs/S_ItemDetails Structure" :default (struct :`Name` "NSLOCTEXT(\"[BF85C17B4B554B3688E9EAA517D8B116]\", \"DB1C888E4BFF2CC9FBE6FDBBAA5D4FA2\", \"Name\")" :`ShortName` "NSLOCTEXT(\"[BF85C17B4B554B3688E9EAA517D8B116]\", \"85C6E802442254A594317EB89462D967\", \"Short Name\")" :`Description` "NSLOCTEXT(\"[BF85C17B4B554B3688E9EAA517D8B116]\", \"8265655B45FFC04EE3F480A4E72D88B0\", \"Descriptions\")" :`Weight` 1.0 :`Width` 1 :`Height` 1 :`AllowQuickBind` true :`AllowDroppingItem` true :`MaxStack` 1 :`WorldActions` (struct :`(WorldActions` "NewEnumerator1,ActionName_15_19BA14C540FCFDAA9B8F29A403079514=NSLOCTEXT(\"[BF85C17B4B554B3688E9EAA517D8B116]\", \"2765D7AB41E66D2FB10894B25327D08F\", \"PICKUP\"))") :`QuickUseAction` "NewEnumerator0" :`WorldClass` "BlueprintGeneratedClass'\"/Game/SurvivalGameKitV2/Blueprints/Items/WorldItems/BP_StaticMasterItem.BP_StaticMasterItem_C\"'" :`IconBackroundColor` (struct :`R` 0.036458 :`G` 0.036458 :`B` 0.036458 :`A` 0.8) :`UIDetails` (struct :`InventoryIcon` "Texture2D'\"/Game/SurvivalGameKitV2/Textures/UI/T_NoIcon_UI.T_NoIcon_UI\"'" :`MoveIcon` "Texture2D'\"/Game/SurvivalGameKitV2/Textures/UI/T_NoIcon_UI.T_NoIcon_UI\"'" :`MoveIconSizeOverride` (struct) :`QuickSlotIcon` "Texture2D'\"/Game/SurvivalGameKitV2/Textures/UI/T_NoIcon_UI.T_NoIcon_UI\"'" :`VenderIcon` "Texture2D'\"/Game/SurvivalGameKitV2/Textures/UI/T_NoIcon_UI.T_NoIcon_UI\"'" :`EquipmentSlotIcon` "Texture2D'\"/Game/SurvivalGameKitV2/Textures/UI/T_NoIcon_UI.T_NoIcon_UI\"'" :`WeaponSlotIcon` "Texture2D'\"/Game/SurvivalGameKitV2/Textures/UI/T_NoIcon_UI.T_NoIcon_UI\"'") :`EquipmentDetails` (struct :`ThirdPersonEquipmentMeshes` (struct) :`FirstPersonBodyEquipmentMeshes` (struct) :`FirstPersonArmsEquipmentMeshes` (struct) :`EquipmentDurabilityReductions` "((NewEnumerator3, 1.000000))") :`ContainerDetails` (struct :`ContainerInventoryCells` 20 :`ContainerColumns` 10 :`UseWeight` true :`MaxWeight` 10.0 :`ContainerRestrictionType` "NewEnumerator0" :`ContainerType` "NewEnumerator1" :`AllowContainerWindow` true :`ItemCountLimit` 1 :`CustomGridLayout` (struct :`DataTable` "CompositeDataTable'\"/Game/SurvivalGameKitV2/Blueprints/Items/MasterLists/MasterGridLayoutList.MasterGridLayoutList\"'")) :`HoldableDetails` (struct :`HoldableSlotSockets` "((NewEnumerator1, \"PrimarySocket\"),(NewEnumerator2, \"SecondarySocket\"))") :`ConsumableDetails` (struct :`ReplaceItem` (struct) :`ReplaceItemAmount` 1) :`AttachmentDetails` (struct) :`AmmoDetails` (struct :`Damage` (struct :`(MinDamage` "1,MaxDamage_8_7DD7F70346375F8E67AC26A5AFD38F8C=1)" :`(Hitbox` "NewEnumerator0,MinDamage_7_AECE5FF040B9D2B3780369BB50422599=1,MaxDamage_8_7DD7F70346375F8E67AC26A5AFD38F8C=1)" :`(Hitbox` "NewEnumerator1,MinDamage_7_AECE5FF040B9D2B3780369BB50422599=1,MaxDamage_8_7DD7F70346375F8E67AC26A5AFD38F8C=1)" :`(Hitbox` "NewEnumerator2,MinDamage_7_AECE5FF040B9D2B3780369BB50422599=1,MaxDamage_8_7DD7F70346375F8E67AC26A5AFD38F8C=1)" :`(Hitbox` "NewEnumerator3,MinDamage_7_AECE5FF040B9D2B3780369BB50422599=1,MaxDamage_8_7DD7F70346375F8E67AC26A5AFD38F8C=1)" :`(Hitbox` "NewEnumerator4,MinDamage_7_AECE5FF040B9D2B3780369BB50422599=1,MaxDamage_8_7DD7F70346375F8E67AC26A5AFD38F8C=1)" :`(Hitbox` "NewEnumerator5,MinDamage_7_AECE5FF040B9D2B3780369BB50422599=1,MaxDamage_8_7DD7F70346375F8E67AC26A5AFD38F8C=1)") :`ProjectileSpeed` 13000.0 :`DamageType` "NewEnumerator3") :`DurabilityDetails` (struct :`DecayDetails` (struct :`DecayTimeMinutes` 30 :`ReplacementItem` (struct :`DataTable` "CompositeDataTable'\"/Game/SurvivalGameKitV2/Blueprints/Items/MasterLists/MasterItemList.MasterItemList\"'"))) :`RecipeDetails` (struct) :`BuildPartDetails` (struct :`DataTable` "CompositeDataTable'\"/Game/SurvivalGameKitV2/Blueprints/Items/MasterLists/MasterBuildPartList.MasterBuildPartList\"'") :`ItemOffsets` (struct :`Rotation` (struct :`W` 1.0) :`Translation` (0.0 0.0 0.0) :`Scale3D` (1.0 1.0 1.0)))))
  (bind ((`ShortName_53_3FDED9954C8DBFC313F77D9D147163D6` _shortname) (`ItemOffsets_94_00D968744A67B380EF0ADAB62D803A4C` _itemoffsets)) (break `/Game/SurvivalGameKitV2/Blueprints/Other/Structs/S_ItemDetails` (`local.ItemDetailsL`)))
  (bind (_itemfound _itemdetails) (`/Game/SurvivalGameKitV2/Blueprints/Other/Interfaces/BP_SGKFunctions.SGK ItemDetails` (`self.TempItem`)))
  (bind (_itemfound_2 _itemdetails_2) (`/Game/SurvivalGameKitV2/Blueprints/Other/Interfaces/BP_SGKFunctions.SGK ItemDetails` (`self.InvItem`)))
  ;[1 1 1] If inv item isnt valid use temp item details
  (if _itemfound_2
    (set `local.ItemDetailsL` _itemdetails_2)
    ;[1 1 1] Apply offset from item list to world item
    (if (not (== _itemoffsets (`KismetMathLibrary.MakeTransform` (0.0 0.0 0.0)))) :!label _label
      (`self.K2_SetActorRotation` (.rotation _itemoffsets))
      (`self.K2_SetActorLocation` (+ (`self.K2_GetActorLocation`) (.location _itemoffsets))))
    (elif _itemfound
      (set `local.ItemDetailsL` _itemdetails)
      (goto _label))))

(fn `Learn`
  (params (PlayerInventory :type "/Game/SurvivalGameKitV2/Blueprints/Components/BP_PlayerInventory Object Reference"))
  ;[1 1 1] Attempt to learn recipes
  (bind _recipelearnt (`/Game/SurvivalGameKitV2/Blueprints/Components/BP_PlayerInventory.LearnAllItemRecipes` (`local.PlayerInventory`) (`self.InvItem`)))
  (if _recipelearnt
    ;[1 1 1] If recipe learned check if should destroy
    (if (`.DestroyItemWhenLearnt_6_691566574CFE133DD707E5A0169D1780` (break `/Game/SurvivalGameKitV2/Blueprints/Other/Structs/S_RecipeDetails` (`.ItemRecipeDetails` (`/Game/SurvivalGameKitV2/Blueprints/Other/Interfaces/BP_SGKFunctions.SGK ItemRecipeDetails` (`self.InvItem`)))))
      (`self.K2_DestroyActor`))))

(fn `Open`
  (params (PlayerInventory :type "/Game/SurvivalGameKitV2/Blueprints/Components/BP_PlayerInventory Object Reference"))
  (bind ((`MasterInventory_8_17FFB7D341FAF2689C1BABA12E3BA9F5` _masterinventory)) (break `/Game/SurvivalGameKitV2/Blueprints/Other/Structs/S_InvItem` (`self.InvItem`)))
  ;[1 1 1] If item has container open UI
  (`/Engine/EditorBlueprintResources/StandardMacros.IsValid` _masterinventory
    (:`Is Valid`
      (`/Game/SurvivalGameKitV2/Blueprints/Components/BP_PlayerInventory.ServerOpenContainerWindow` (`local.PlayerInventory`) _masterinventory true))))

(fn `Pickup`
  (params (PlayerInventory :type "/Game/SurvivalGameKitV2/Blueprints/Components/BP_PlayerInventory Object Reference"))
  (locals (StartAmountL :type Integer))
  (bind (_invitem_id _invitem_amount _invitem_masterinventory) (break `/Game/SurvivalGameKitV2/Blueprints/Other/Structs/S_InvItem` (`self.InvItem`)))
  ;[1 1 1] Set start amount
  (set `local.StartAmountL` (`.Amount_5_62DB2267439500D86A52E0B2266494D2` (break `/Game/SurvivalGameKitV2/Blueprints/Other/Structs/S_InvItem` (`self.InvItem`))))
  ;[1 1 1] Close other players using the inventory
  (`/Engine/EditorBlueprintResources/StandardMacros.IsValid` _invitem_masterinventory
    (:`Is Valid`
      (`/Game/SurvivalGameKitV2/Blueprints/Components/BP_MasterInventory.CloseOtherPlayerTabs` _invitem_masterinventory null))
    (:`Is Not Valid`
      _))
  ;[1 1 1] Attempt to pickup item and add to inventory if added play pick up sound and destroy actor
  (bind (_remainingitem _remaininginvitem) (`/Game/SurvivalGameKitV2/Blueprints/Components/BP_PlayerInventory.AttemptToAddItem` (`local.PlayerInventory`) (`self.InvItem`) true true))
  (if _remainingitem
    (bind _output_get (set `self.InvItem` _remaininginvitem))
    (bind _output_get_2 (set `self.TempItem` _output_get))
    ;[1 1 1] If remaining items left check if same as start and if not play pickup sound
    (if (not (== (`.Amount_5_62DB2267439500D86A52E0B2266494D2` (break `/Game/SurvivalGameKitV2/Blueprints/Other/Structs/S_InvItem` _output_get_2)) (`local.StartAmountL`)))
      (`/Game/SurvivalGameKitV2/Blueprints/Components/BP_MasterInventory.SGK ItemSound` (`local.PlayerInventory`) (`.ID_2_84C2CB8945979246059C568DCD463423` (break `/Game/SurvivalGameKitV2/Blueprints/Other/Structs/S_InvItem` (`self.InvItem`))) "NewEnumerator12"))
    (else
      (`/Game/SurvivalGameKitV2/Blueprints/Components/BP_MasterInventory.SGK ItemSound` (`local.PlayerInventory`) (`.ID_2_84C2CB8945979246059C568DCD463423` (break `/Game/SurvivalGameKitV2/Blueprints/Other/Structs/S_InvItem` (`self.InvItem`))) "NewEnumerator12")
      (`self.K2_DestroyActor`))))

(fn `SGK AllowInteraction`
  (returns (AllowInteraction :type Boolean))
  (return true))

(fn `SGK CodeCheck`
  (params (Code :type Text))
  (returns (CodeAccepted :type Boolean))
  (return false))

(fn `SGK DropItem`
  (params (InvItem :type "/Game/SurvivalGameKitV2/Blueprints/Other/Structs/S_InvItem Structure") (Dropped :type Boolean) (Spawned :type Boolean) (SaveLoaded :type Boolean))
  (returns (ReturnValue :type Boolean))
  (locals (ItemL :type "/Game/SurvivalGameKitV2/Blueprints/Other/Structs/S_InvItem Structure"))
  (bind ((`MasterInventory_8_17FFB7D341FAF2689C1BABA12E3BA9F5` _masterinventory)) (break `/Game/SurvivalGameKitV2/Blueprints/Other/Structs/S_InvItem` (`local.ItemL`)))
  (set `self.Dropped` Dropped)
  (set `self.Spawned` Spawned)
  (set `self.SaveGameLoaded` SaveLoaded)
  (set `local.ItemL` InvItem)
  (if (or (`KismetSystemLibrary.IsStandalone`) (`local.Dropped`) (`local.Spawned`))
    (if (`KismetSystemLibrary.IsStandalone`)
      (set `self.InvItem` (`local.ItemL`) :!label _label)
      (else
        (`/Engine/EditorBlueprintResources/StandardMacros.IsValid` _masterinventory
          (:`Is Valid`
            (if (`ActorComponent.bReplicates` _masterinventory)
              (goto _label)
              (else
                (setmembers `/Game/SurvivalGameKitV2/Blueprints/Other/Structs/S_InvItem` :`StructRef` (`local.ItemL`) :`MasterInventory` null)
                (goto _label))))
          (:`Is Not Valid`
            (set `self.InvItem` (`local.ItemL`)))))))
  (set `self.TempItem` InvItem)
  (if (or (`self.Dropped`) (`self.Spawned`))
    (`self.ItemOffsets`)
    (if (`self.Spawned`)
      _
      (elif (`self.UseDroppedItemDestroyTimer`)
        (`KismetSystemLibrary.K2_SetTimerDelegate` (`|CreateDelegate` :!event `DropDestroyTimer`) (`self.DropDestroyTime`)))))
  (`StaticMeshComponent.SetStaticMesh` (`self.StaticMesh`) (`.StaticMesh_30_DB8565E8487831578F6D18823B88B876` (break `/Game/SurvivalGameKitV2/Blueprints/Other/Structs/S_ItemDetails` (`.ItemDetails` (`/Game/SurvivalGameKitV2/Blueprints/Other/Interfaces/BP_SGKFunctions.SGK ItemDetails` (`self.TempItem`))))))
  (return true))

(fn `SGK EndHighlight`
  (returns (ReturnValue :type Boolean))
  (return false))

(fn `SGK EndInteraction`
  (params (PlayerInventory :type "/Game/SurvivalGameKitV2/Blueprints/Components/BP_PlayerInventory Object Reference"))
  (returns (ReturnValue :type Boolean))
  (return false))

(fn `SGK GetVerifiedPlayers`
  (returns (VerifiedPlayers :type "Array of Text"))
  (return))

(fn `SGK Interact`
  (params (PlayerInventory :type "/Game/SurvivalGameKitV2/Blueprints/Components/BP_PlayerInventory Object Reference") (Action :type "/Game/SurvivalGameKitV2/Blueprints/Other/Enum/E_WorldActions Enum" :default "NewEnumerator0"))
  (returns (ReturnValue :type Boolean))
  (`self.InteractActions` PlayerInventory Action)
  (return true))

(fn `SGK InteractName`
  (returns (InteractName :type Text))
  (return (`.Name_26_D03100674B3BD75EEF9FD9A1E4F9CC34` (break `/Game/SurvivalGameKitV2/Blueprints/Other/Structs/S_ItemDetails` (`.ItemDetails` (`/Game/SurvivalGameKitV2/Blueprints/Other/Interfaces/BP_SGKFunctions.SGK ItemDetails` (`self.InvItem`)))))))

(fn `SGK InvItem`
  (returns (IsItem :type Boolean) (InvItem :type "/Game/SurvivalGameKitV2/Blueprints/Other/Structs/S_InvItem Structure"))
  (locals (CombineItemsL :type "/Game/SurvivalGameKitV2/Blueprints/Other/Structs/S_InvItem Structure"))
  (bind _output_get (set `local.CombineItemsL` (`self.InvItem`)))
  (bind _structout (setmembers `/Game/SurvivalGameKitV2/Blueprints/Other/Structs/S_InvItem` :`StructRef` _output_get :`MasterInventory` (`.MasterInventory_8_17FFB7D341FAF2689C1BABA12E3BA9F5` (break `/Game/SurvivalGameKitV2/Blueprints/Other/Structs/S_InvItem` (`self.TempItem`)))))
  (return true _structout))

(fn `SGK ItemAmount`
  (returns (Amount :type Integer))
  (return (`.Amount_5_62DB2267439500D86A52E0B2266494D2` (break `/Game/SurvivalGameKitV2/Blueprints/Other/Structs/S_InvItem` (`self.InvItem`)))))

(fn `SGK Mesh`
  (returns (Mesh :type "PrimitiveComponent Object Reference"))
  (return null))

(fn `SGK PossibleActions`
  (params (PlayerInventory :type "/Game/SurvivalGameKitV2/Blueprints/Components/BP_PlayerInventory Object Reference"))
  (returns (ActionsFound :type Boolean) (PossibleActions :type "Array of /Game/SurvivalGameKitV2/Blueprints/Other/Structs/S_WorldAction Structure"))
  (bind ((`ShortName_53_3FDED9954C8DBFC313F77D9D147163D6` _shortname) (`AllowQuickBind_65_ABE4ABEB4EC0B8EC89B4A9A18E208874` _allowquickbind) (`AllowDroppingItem_67_10BDCFBC4E21AD7EE24CE79692B3342C` _allowdroppingitem) (`InventoryActions_112_685EE89C49954FBB235025AD602B3208` _inventoryactions) (`WorldActions_116_B4CAF39A421B065A46DEACBC5DBD40EE` _worldactions)) (break `/Game/SurvivalGameKitV2/Blueprints/Other/Structs/S_ItemDetails` (`.ItemDetails` (`/Game/SurvivalGameKitV2/Blueprints/Other/Interfaces/BP_SGKFunctions.SGK ItemDetails` (`self.InvItem`)))))
  (return (> (`KismetArrayLibrary.Array_Length` _worldactions) 0) _worldactions))

(fn `SGK StartHighlight`
  (returns (ReturnValue :type Boolean))
  (return false))

(fn `SGK UpdateCode`
  (params (Code :type Text))
  (returns (ReturnValue :type Boolean))
  (return false))

(fn `SGK VerifyPlayer`
  (params (Text :type Text))
  (returns (ReturnValue :type Boolean))
  (return false))

(fn `UserConstructionScript`
  (bind (_item_datatable _item_rowname) (break `DataTableRowHandle` (`self.Item`)))
  (bind (_item_datatable_2 _item_rowname_2) (break `DataTableRowHandle` (`self.Item`)))
  (bind (_item_datatable_3 _item_rowname_3) (break `DataTableRowHandle` (`self.Item`)))
  (set `self.RefreshItem` false)
  (if (or (`self.Spawned`) (`self.Dropped`) (`self.SaveGameLoaded`))
    (`StaticMeshComponent.SetStaticMesh` (`self.StaticMesh`) (`.StaticMesh_30_DB8565E8487831578F6D18823B88B876` (break `/Game/SurvivalGameKitV2/Blueprints/Other/Structs/S_ItemDetails` (`.ItemDetails` (`/Game/SurvivalGameKitV2/Blueprints/Other/Interfaces/BP_SGKFunctions.SGK ItemDetails` (`self.InvItem`))))))
    (else
      (if (!= _item_rowname_3 (`.ID_2_84C2CB8945979246059C568DCD463423` (break `/Game/SurvivalGameKitV2/Blueprints/Other/Structs/S_InvItem` (`self.InvItem`))))
        (setmembers `/Game/SurvivalGameKitV2/Blueprints/Other/Structs/S_InvItem` :`StructRef` (`self.InvItem`) :`ID` _item_rowname :`Amount` (`self.ItemAmount`))
        (`self.ItemOffsets`)
        (else
          (setmembers `/Game/SurvivalGameKitV2/Blueprints/Other/Structs/S_InvItem` :`StructRef` (`self.InvItem`) :`ID` _item_rowname_2 :`Amount` (`self.ItemAmount`))))
      (`StaticMeshComponent.SetStaticMesh` (`self.StaticMesh`) (`.StaticMesh_30_DB8565E8487831578F6D18823B88B876` (break `/Game/SurvivalGameKitV2/Blueprints/Other/Structs/S_ItemDetails` (`.ItemDetails` (`/Game/SurvivalGameKitV2/Blueprints/Other/Interfaces/BP_SGKFunctions.SGK ItemDetails` (`self.InvItem`)))))))))