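; Character component for one foot socket that plays surface-dependent footstep sounds, particles and decals, and optionally computes foot IK.
; Socket and footstep data load from an overridable DataTable preset.
; ProcessFootstep line-traces the surface's physical material, lets BP_SurfaceOverrider_Base actors override it, detects splashes, then looks up effects by footstep and surface type.
; With IK enabled, Tick traces the ground to interpolate clamped bone rotation and height offset.
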(event `self.ReceiveBeginPlay`
  ;[1 1 1] Begin play event checks footstep component settings.
  (`self.InitializeComponent`))

(event `self.ReceiveTick`
  (params (DeltaSeconds :type "Float (single-precision)"))
  ;[1 1 1] Update variables for foot IK.
  (if (`self.IK_Enabled`)
    (`self.UpdateFootIK`)))

(fn `CheckOverriddenSurface`
  (params (Location :type "Vector Structure"))
  (returns (Overridden :type Boolean) (SurfaceType :type "EPhysicalSurface Enum") (PlaySplash :type Boolean))
  ;[1 1 1] Check and return overridden surface information in target location.
  (bind (_outhits _returnvalue) (`KismetSystemLibrary.SphereTraceMultiForObjects` Location (+ Location 0.1) 1.0 (`|MakeArray` "ObjectTypeQuery10" :!type "EObjectTypeQuery Enum")))
  (if _returnvalue
    (bind _asbp_surface_overrider_base (cast `/Game/EasyFootstepSystem/Blueprints/SurfaceActors/BP_SurfaceOverrider_Base` (`.HitActor` (`GameplayStatics.BreakHitResult` (`|GetArrayItem` _outhits))))
      (:`then`
        (return true (`/Game/EasyFootstepSystem/Blueprints/SurfaceActors/BP_SurfaceOverrider_Base.SurfaceType` _asbp_surface_overrider_base) (`/Game/EasyFootstepSystem/Blueprints/SurfaceActors/BP_SurfaceOverrider_Base.PlaySplash` _asbp_surface_overrider_base)))
      (:`CastFailed`
        _)))
  (return false "SurfaceType_Default" false))

(fn `CheckSurface`
  (params (FootstepType :type "/Game/EasyFootstepSystem/Blueprints/Enumerations/E_FootstepType Enum" :default "NewEnumerator0"))
  (returns (HasSurface :type Boolean) (Location :type "Vector Structure") (Surface :type "EPhysicalSurface Enum") (PlaySplash :type Boolean))
  (locals (LocalLocation :type "Vector Structure" :default (0.0 0.0 0.0)) (LocalSurfaceType :type "EPhysicalSurface Enum") (LocalPlaySplash :type Boolean))
  ;[1 1 1] Check surface under foot and return surface information.
  (bind _location (`self.GetFootLocation`))
  (bind _output_get (set `local.LocalLocation` _location))
  (bind (_outhit _returnvalue) (`KismetSystemLibrary.LineTraceSingle` (+ _output_get (0.0 0.0 20.0)) (- _output_get (select `bool` (`|EnumEquality` FootstepType "NewEnumerator3") :`false` (0.0 0.0 30.0) :`true` (0.0 0.0 60.0) :!type "Vector Structure")) "TraceTypeQuery1"))
  (if _returnvalue
    (bind (_bblockinghit _binitialoverlap _time _distance _location_2 _impactpoint _normal _impactnormal _physmat) (`GameplayStatics.BreakHitResult` _outhit))
    (set `local.LocalSurfaceType` (`PhysicalMaterial.SurfaceType` _physmat))
    (bind _output_get_2 (set `local.LocalLocation` _location_2))
    (bind (_overridden _surfacetype _playsplash) (`self.CheckOverriddenSurface` _output_get_2))
    (if _overridden
      (set `local.LocalSurfaceType` _surfacetype)
      (set `local.LocalPlaySplash` _playsplash)
      (else
        (bind (_outhit_2 _returnvalue_2) (`KismetSystemLibrary.LineTraceSingleForObjects` (+ _output_get_2 (0.0 0.0 150.0)) (- _output_get_2 (0.0 0.0 15.0)) (`|MakeArray` "ObjectTypeQuery10" :!type "EObjectTypeQuery Enum") true))
        (set `local.LocalPlaySplash` _returnvalue_2)))
    (return true (`local.LocalLocation`) (`local.LocalSurfaceType`) (`local.LocalPlaySplash`))
    (else
      (return false (0.0 0.0 0.0) "SurfaceType_Default" false))))

(fn `ClearOverriddenFootstepsPreset`
  ;[1 1 1] Clear overridden footstep preset handle and set default component settings.
  (set `self.OverriddenFootstepsPresetHandle` (struct))
  (set `self.FootstepsPresetOverridden` false)
  (`self.InitializeComponent`))

(fn `FindFootstepSurfaceData`
  (params (FootstepType :type "/Game/EasyFootstepSystem/Blueprints/Enumerations/E_FootstepType Enum" :default "NewEnumerator0") (SurfaceType :type "EPhysicalSurface Enum" :default "SurfaceType_Default"))
  (returns (Found :type Boolean) (FootstepSurfaceData :type "/Game/EasyFootstepSystem/Blueprints/Structures/STR_FootstepSurfaceData Structure"))
  (locals (LocalFootstepType :type "/Game/EasyFootstepSystem/Blueprints/Enumerations/E_FootstepType Enum" :default "NewEnumerator0") (LocalSurfaceType :type "EPhysicalSurface Enum") (LocalFootstepSurfaceData :type "/Game/EasyFootstepSystem/Blueprints/Structures/STR_FootstepSurfaceData Structure"))
  ;[1 1 1] Try to find footstep surface data from footsteps data depending on footstep and surface types.
  (set `local.LocalFootstepType` FootstepType)
  (set `local.LocalSurfaceType` SurfaceType)
  (for _array_element (`self.FootstepsData`)
    (bind (_footsteptype _footstepsurfacesdata) (break `/Game/EasyFootstepSystem/Blueprints/Structures/STR_FootstepTypeData` _array_element))
    (if (== _footsteptype (`local.LocalFootstepType`))
      (for _array_element_2 _footstepsurfacesdata
        (bind _returnvalue (== (`.SurfaceType_2_0B4AC8254A593591631BFFB22454DBD6` (break `/Game/EasyFootstepSystem/Blueprints/Structures/STR_FootstepSurfaceData` _array_element_2)) (`local.LocalSurfaceType`)))
        (if _returnvalue
          (return _returnvalue _array_element_2)))))
  (return false))

(fn `GetFootLocation`
  (returns (Location :type "Vector Structure"))
  ;[1 1 1] Returns foot location.
  (return (`SceneComponent.GetSocketLocation` (`self.SkeletalMeshReference`) (`self.FootSocket`))))

(fn `InitializeComponent`
  (locals (LocalPresetHandle :type "DataTableRowHandle Structure" :default (struct)))
  ;[1 1 1] Try to load footstep component settings from datatable and check it.
  (bind _ascharacter (cast `Character` (`self.GetOwner`))
    (:`then`
      (set `self.SkeletalMeshReference` (`Character.Mesh` _ascharacter))
      (bind _output_get (set `local.LocalPresetHandle` (select `bool` (`self.FootstepsPresetOverridden`) :`false` (`self.FootstepsPresetHandle`) :`true` (`self.OverriddenFootstepsPresetHandle`))))
      (bind (_datatable _rowname) (break `DataTableRowHandle` _output_get))
      (`/Engine/EditorBlueprintResources/StandardMacros.IsValid` _datatable
        (:`Is Valid`
          (bind _returnvalue (`|GetDataTableRow` _datatable _rowname)
            (:`then`
              (bind (_footsocket _footstepsdata) (break `/Game/EasyFootstepSystem/Blueprints/Structures/STR_FootstepSettings` _returnvalue))
              (set `self.FootSocket` _footsocket)
              (set `self.FootstepsData` _footstepsdata)
              (if (not (`SceneComponent.DoesSocketExist` (`self.SkeletalMeshReference`) (`self.FootSocket`)))
                (`KismetSystemLibrary.PrintText` (`|FormatText` "Wrong footstep settings in {ClassName} class!" (`KismetTextLibrary.Conv_StringToText` (`KismetSystemLibrary.GetClassDisplayName` (`GameplayStatics.GetObjectClass` (`self.GetOwner`))))) true true (struct :`R` 1.0 :`A` 1.0) 10.0 :!label _label)))
            (:`RowNotFound`
              (goto _label))))))
    (:`CastFailed`
      (goto _label))))

(fn `PlayFootstepSounds`
  (params (Location :type "Vector Structure") (FootstepSurfaceData :type "/Game/EasyFootstepSystem/Blueprints/Structures/STR_FootstepSurfaceData Structure") (PlaySplash :type Boolean))
  (locals (LocalLocation :type "Vector Structure") (LocalSurfaceData :type "/Game/EasyFootstepSystem/Blueprints/Structures/STR_FootstepSurfaceData Structure") (LocalPlaySplash :type Boolean))
  (bind ((`SplashSound_7_778BBF104A936D00CB640B9877E67548` _splashsound)) (break `/Game/EasyFootstepSystem/Blueprints/Structures/STR_FootstepSurfaceData` (`local.LocalSurfaceData`)))
  (bind ((`SurfaceSound_8_F50C176145232D8481A6DF8ACE86A71E` _surfacesound)) (break `/Game/EasyFootstepSystem/Blueprints/Structures/STR_FootstepSurfaceData` (`local.LocalSurfaceData`)))
  ;[1 1 1] Play footstep sounds in target location depending on footstep surface data.
  (set `local.LocalLocation` Location)
  (set `local.LocalSurfaceData` FootstepSurfaceData)
  (set `local.LocalPlaySplash` PlaySplash)
  (`|ExecutionSequence`
    (:`then_0`
      (`/Engine/EditorBlueprintResources/StandardMacros.IsValid` _surfacesound
        (:`Is Valid`
          (`GameplayStatics.PlaySoundAtLocation` _surfacesound (`local.LocalLocation`) (struct) (select `bool` (`local.LocalPlaySplash`) :`false` 1.0 :`true` 0.65 :!type "Float (single-precision)") 1.0 0.0 null null null))))
    (:`then_1`
      (if (`local.LocalPlaySplash`)
        (`/Engine/EditorBlueprintResources/StandardMacros.IsValid` _splashsound
          (:`Is Valid`
            (`GameplayStatics.PlaySoundAtLocation` _splashsound (`local.LocalLocation`) (struct) 1.0 1.0 0.0 null null null)))))))

(fn `ProcessFootstep`
  (params (FootSocket :type Name) (FootstepType :type "/Game/EasyFootstepSystem/Blueprints/Enumerations/E_FootstepType Enum" :default "NewEnumerator0") (PlaySounds :type Boolean) (SpawnEffects :type Boolean))
  (locals (LocalFootstepType :type "/Game/EasyFootstepSystem/Blueprints/Enumerations/E_FootstepType Enum" :default "NewEnumerator0") (LocalPlaySounds :type Boolean) (LocalSpawnEffects :type Boolean) (LocalLocation :type "Vector Structure" :default (0.0 0.0 0.0)) (LocalSurface :type "EPhysicalSurface Enum" :default "SurfaceType_Default") (LocalPlaySplash :type Boolean :default false) (LocalSurfaceData :type "/Game/EasyFootstepSystem/Blueprints/Structures/STR_FootstepSurfaceData Structure"))
  ;[1 1 1] Process footstep event, spawn effects and play sounds depending on footstep and surface types.
  (`/Engine/EditorBlueprintResources/StandardMacros.IsValid` (`self.SkeletalMeshReference`)
    (:`Is Valid`
      (if (== FootSocket (`self.FootSocket`))
        (bind _output_get (set `local.LocalFootstepType` FootstepType))
        (set `local.LocalPlaySounds` PlaySounds)
        (set `local.LocalSpawnEffects` SpawnEffects)
        (bind (_hassurface _location _surface _playsplash) (`self.CheckSurface` _output_get))
        (if _hassurface
          (set `local.LocalLocation` _location)
          (set `local.LocalSurface` _surface)
          (set `local.LocalPlaySplash` _playsplash)
          (bind (_found _footstepsurfacedata) (`self.FindFootstepSurfaceData` (`local.LocalFootstepType`) (`local.LocalSurface`)))
          (if _found
            (set `local.LocalSurfaceData` _footstepsurfacedata)
            (`|ExecutionSequence`
              (:`then_0`
                (if (`local.LocalPlaySounds`)
                  (`self.PlayFootstepSounds` (`local.LocalLocation`) (`local.LocalSurfaceData`) (`local.LocalPlaySplash`))))
              (:`then_1`
                (if (`local.LocalSpawnEffects`)
                  (`self.SpawnFootstepEffects` (`local.LocalLocation`) (`local.LocalSurfaceData`) (`local.LocalPlaySplash`)))))))))))

(fn `SetOverriddenFootstepsPreset`
  (params (FootstepsPresetHandle :type "DataTableRowHandle Structure"))
  ;[1 1 1] Set overridden footstep preset handle and load component settings from datatable.
  (bind _output_get (set `self.OverriddenFootstepsPresetHandle` FootstepsPresetHandle))
  (bind (_datatable _rowname) (break `DataTableRowHandle` _output_get))
  (set `self.FootstepsPresetOverridden` (and (`KismetSystemLibrary.IsValid` _datatable) (!= _rowname "None")))
  (`self.InitializeComponent`))

(fn `SpawnFootstepEffects`
  (params (Location :type "Vector Structure") (FootstepSurfaceData :type "/Game/EasyFootstepSystem/Blueprints/Structures/STR_FootstepSurfaceData Structure") (PlaySplash :type Boolean))
  (locals (LocalLocation :type "Vector Structure") (LocalSurfaceData :type "/Game/EasyFootstepSystem/Blueprints/Structures/STR_FootstepSurfaceData Structure") (LocalPlaySplash :type Boolean) (LocalParticle :type "ParticleSystem Object Reference"))
  (bind ((`DecalMaterial_14_4A90C14B45DB3DFFED0E2CA8D26DA500` _decalmaterial) (`DecalSize_17_DF714A214ADC161404E6058F6BAB9FF4` _decalsize) (`DecalLifeSpan_20_8D07CD6C4E71AAB33AACE3AFFDE235FF` _decallifespan)) (break `/Game/EasyFootstepSystem/Blueprints/Structures/STR_FootstepSurfaceData` (`local.LocalSurfaceData`)))
  (bind ((`SurfaceParticle_21_D8D385474F5FAD746C1F5D8DD7B28232` _surfaceparticle) (`SplashParticle_24_72D5C5254A1C45327DF0D789091BCC7B` _splashparticle)) (break `/Game/EasyFootstepSystem/Blueprints/Structures/STR_FootstepSurfaceData` (`local.LocalSurfaceData`)))
  ;[1 1 1] Spawn footstep effects in target location depending on footstep surface data.
  (set `local.LocalLocation` Location)
  (set `local.LocalSurfaceData` FootstepSurfaceData)
  (set `local.LocalPlaySplash` PlaySplash)
  (`|ExecutionSequence`
    (:`then_0`
      (bind _output_get (set `local.LocalParticle` (select `bool` (`local.LocalPlaySplash`) :`false` _surfaceparticle :`true` _splashparticle)))
      (`/Engine/EditorBlueprintResources/StandardMacros.IsValid` _output_get
        (:`Is Valid`
          (`GameplayStatics.SpawnEmitterAtLocation` (`local.LocalParticle`) (`local.LocalLocation`)))))
    (:`then_1`
      (if (not (`local.LocalPlaySplash`))
        (`/Engine/EditorBlueprintResources/StandardMacros.IsValid` _decalmaterial
          (:`Is Valid`
            (`GameplayStatics.SpawnDecalAtLocation` _decalmaterial _decalsize (`local.LocalLocation`) (`KismetMathLibrary.MakeRotator` 90.0 -90.0 (.yaw (`Actor.K2_GetActorRotation` (`self.GetOwner`)))) _decallifespan)))))))

(fn `UpdateFootIK`
  (bind _skeletalmeshreference (`self.SkeletalMeshReference`))
  (bind (_returnvalue_x _returnvalue_y _returnvalue_z) (`KismetMathLibrary.BreakVector` (`SceneComponent.K2_GetComponentLocation` _skeletalmeshreference)))
  (bind (_x _y) (`KismetMathLibrary.BreakVector2D` (`self.IK_TraceOffsets`)))
  (bind (_returnvalue_x_2 _returnvalue_y_2) (`KismetMathLibrary.BreakVector` (`SceneComponent.GetSocketLocation` _skeletalmeshreference (`self.FootSocket`))))
  ;[1 1 1] Update foot IK variables.
  (`/Engine/EditorBlueprintResources/StandardMacros.IsValid` _skeletalmeshreference
    (:`Is Valid`
      (bind _outhit (`KismetSystemLibrary.LineTraceSingle` (`KismetMathLibrary.MakeVector` _returnvalue_x_2 _returnvalue_y_2 (+ _returnvalue_z _x)) (`KismetMathLibrary.MakeVector` _returnvalue_x_2 _returnvalue_y_2 (- _returnvalue_z _y)) "TraceTypeQuery1"))
      (if (`GameplayStatics.BreakHitResult` _outhit)
        (set `self.IK_BoneTargetRotation` (`KismetMathLibrary.MakeRotator` (`KismetMathLibrary.FClamp` (`KismetMathLibrary.DegAtan2` (.y (`.Normal` (`GameplayStatics.BreakHitResult` _outhit))) (.z (`.Normal` (`GameplayStatics.BreakHitResult` _outhit)))) -10.0 10.0) (* (`KismetMathLibrary.FClamp` (`KismetMathLibrary.DegAtan2` (.x (`.Normal` (`GameplayStatics.BreakHitResult` _outhit))) (.z (`.Normal` (`GameplayStatics.BreakHitResult` _outhit)))) -30.0 30.0) -1.0)))
        (set `self.IK_BoneTargetTranslation` (`KismetMathLibrary.FClamp` (- (.z (`.Location` (`GameplayStatics.BreakHitResult` _outhit))) _returnvalue_z) -30.0 20.0))
        (else
          (set `self.IK_BoneTargetRotation` (struct))
          (set `self.IK_BoneTargetTranslation` 0.0)))
      (set `self.IK_BoneRotation` (`KismetMathLibrary.RInterpTo` (`self.IK_BoneRotation`) (`self.IK_BoneTargetRotation`) 0.0 (`self.IK_BoneRotationInterpSpeed`)))
      (set `self.IK_BoneTranslation` (`KismetMathLibrary.FInterpTo` (`self.IK_BoneTranslation`) (`self.IK_BoneTargetTranslation`) (`GameplayStatics.GetWorldDeltaSeconds`) (`self.IK_BoneTranslationInterpSpeed`))))))